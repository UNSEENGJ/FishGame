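; BP_TPGameMode is a match-state game mode that controls match start and end and shows the outcome screen.
; ReadyToStartMatch and ReadyToEndMatch simply return the StartMatch and MatchEnded variables.
; BeginPlay plays a 2D sound cue.
; ShowResultWindow switches on GetGameResult (Trash, Perfect or Hmm) to add the matching outro overlay widget to the viewport.
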(event `self.ReceiveBeginPlay`
  (`GameplayStatics.PlaySound2D` "/Game/Asset/Sound/NewSoundCue.NewSoundCue" 1.0 1.0 0.0 null null))

(event `self.ShowResultWindow`
  (bind _returnvalue (`self.GetGameResult`))
  (switch `ETPGameResult` _returnvalue
    (:`ETPGameResult_Trash`
      (bind _returnvalue_2 (`|CreateWidget` "/Game/Blueprint/Widget/BPW_OutroOverlay1.BPW_OutroOverlay1_C"))
      (`UserWidget.AddToViewport` _returnvalue_2 0))
    (:`ETPGameResult_Perfect`
      (bind _returnvalue_3 (`|CreateWidget` "/Game/Blueprint/Widget/BPW_OutroOverlay2.BPW_OutroOverlay2_C"))
      (`UserWidget.AddToViewport` _returnvalue_3 0))
    (:`ETPGameResult_Hmm`
      (bind _returnvalue_4 (`|CreateWidget` "/Game/Blueprint/Widget/BPW_OutroOverlay3.BPW_OutroOverlay3_C"))
      (`UserWidget.AddToViewport` _returnvalue_4 0))))

(fn `ReadyToEndMatch`
  (returns (ReturnValue :type Boolean))
  (return (`self.bMatchEnded`)))

(fn `ReadyToStartMatch`
  (returns (ReturnValue :type Boolean))
  (return (`self.bStartMatch`)))

(fn `UserConstructionScript`)