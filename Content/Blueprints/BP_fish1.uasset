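; BP_fish1 is a fish actor that appears after a timed wait and drops down to a fixed height.
; BeginPlay caches the skeletal mesh's world location, and a Delay in Tick sets the Time flag after five seconds.
; Tick then shows the mesh and lowers it a fixed step per frame, independent of delta time, until the height limit.
; The BeginPlay delay leads nowhere, and the looping carp animation call is unconnected.
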(event `self.ReceiveBeginPlay`
  (set `self.Location` (`SceneComponent.K2_GetComponentLocation` (`self.SkeletalMesh`)))
  (`KismetSystemLibrary.Delay` 3.0))

(event `self.ReceiveTick`
  (params (DeltaSeconds :type "Float (single-precision)"))
  (bind (_location_x _location_y _location_z) (`KismetMathLibrary.BreakVector` (`self.Location`)))
  (bind (_location_x_2 _location_y_2 _location_z_2) (`KismetMathLibrary.BreakVector` (`self.Location`)))
  (if (`self.time`)
    (`SceneComponent.SetVisibility` (`self.SkeletalMesh`) true false)
    (if (not (<= _location_z_2 80.0))
      (bind _output_get (set `self.Location` (`KismetMathLibrary.MakeVector` _location_x _location_y (`KismetMathLibrary.Conv_IntToDouble` (- _location_z 6))))))
    (`SceneComponent.K2_SetWorldLocation` (`self.SkeletalMesh`) _output_get false false)
    (else
      (`KismetSystemLibrary.Delay` 5.0)
      (set `self.time` true))))

(fn `UserConstructionScript`)